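; Timer actor that displays a countdown on a TextRender component.
; Each Tick writes ActualTime to the text and accumulates delta time, subtracting one from ActualTime and resetting the accumulator when the sum passes one second.
; The count has no lower limit, and the reset discards leftover time.
; BeginPlay enables input from player controller 0, though the graph has no input events.
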(event `self.ReceiveBeginPlay`
  (`self.EnableInput` (`GameplayStatics.GetPlayerController` 0)))

(event `self.ReceiveTick`
  (params (DeltaSeconds :type "Float (single-precision)"))
  (bind _returnvalue (+ DeltaSeconds (`self.Timer`)))
  (`TextRenderComponent.K2_SetText` (`self.TextRender`) (`KismetTextLibrary.Conv_DoubleToText` (`self.ActualTime`) "HalfToEven"))
  (set `self.Timer` _returnvalue)
  (if (> _returnvalue 1.0)
    (set `self.ActualTime` (- (`self.ActualTime`) 1.0))
    (set `self.Timer` 0.0)))

(event `InputAction|1`
  (params (Key :type "Key Structure" :default "AnyKey")))

(fn `UserConstructionScript`)