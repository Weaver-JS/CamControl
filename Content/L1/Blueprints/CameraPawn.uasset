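; CameraPawn is a possessable camera the player looks around from and hops between, with an accuse input that wins or loses on a criminal flag.
; While possessed, a sphere trace shows a prompt on reachable cameras; Space or dwelling gaze triggers fade, sound and possession, turning the new camera toward the old one.
; Reachability is a hardcoded per-level graph keyed on actor names.
; E briefly shows a timer actor.
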(event Collision|EventActorBeginOverlap
  (params (OtherActor :type Actor%20Object%20Reference)))

(event EventUnpossessed
  (params (OldController :type Controller%20Object%20Reference))
  ;[1 1 1] Toggle Visibility of Stiatic Mesh
  (Rendering|SetVisibility (Variables|Default|GetStaticMesh) true false)
  (Variables|Default|SetisPossessed false))

(event EventTick
  (params (DeltaSeconds :type Float%20%28single-precision%29))
  (bind _returnvalue (Transformation|GetActorLocation))
  (bind _actual_timer (Variables|Default|GetActual_Timer))
  (Utilities|FlowControl|Sequence
    (:then_0
      ;[1 1 1] make Text invisible every loop
      (Rendering|SetVisibility (Variables|Default|GetMaterialBillboard) false false)
      ;[1 1 1] Every loop, we check if player looking to Camera to know if we should print the "Space" prompt
      (Rendering|SetVisibility (Variables|Default|GetTextRender) false false))
    (:then_1
      (if (Variables|Default|GetisPossessed)
        (bind _outhit (Collision|SphereTraceForObjects _returnvalue (+ _returnvalue (* (Transformation|GetActorForwardVector (Game|GetPlayerController 0)) 1e+04)) 1.5e+02 (Utilities|Array|MakeArray "ObjectTypeQuery7") false 0 "ForOneFrame"))
        (if (== (Utilities|GetClass (.HitActor (Collision|BreakHitResult _outhit))) "CameraPawn_C")
          (Variables|Default|SetisLooking true)
          (bind _ascamera_pawn (Utilities|Casting|CastToCameraPawn (.HitActor (Collision|BreakHitResult _outhit))))
          ;[1 1 1] Miramos si podemos ir a esa camara
          (bind _canigo (CallFunction|CanWeGotoThatCamera _ascamera_pawn))
          (if _canigo
            (Transformation|SetWorldRotation (Actor|GetComponentbyClass _ascamera_pawn "/Script/Engine.TextRenderComponent") (Math|Rotator|MakeRotfromX (- (Transformation|GetActorLocation) (Transformation|GetWorldLocation (Actor|GetComponentbyClass _ascamera_pawn "/Script/Engine.TextRenderComponent")))) false false)
            (Rendering|SetVisibility (Actor|GetComponentbyClass _ascamera_pawn "/Script/Engine.TextRenderComponent") true false)
            (Rendering|SetVisibility (Actor|GetComponentsByClass _ascamera_pawn "/Script/Engine.MaterialBillboardComponent") true false)
            (if (Variables|Default|GetisLooking)
              (bind _output_get (Variables|Default|SetTimeToteleport (+ (Variables|Default|GetTimeToteleport) DeltaSeconds)))
              (if (>= _output_get 1.5)
                ;[1 1 1] Aqui se activa el FadeOut
                (bind (_newpawn _canwe) (CallFunction|CanWeTransporttoCamera))
                (if _canwe
                  (Variables|Default|SetTimeToteleport -0.2)
                  (Utilities|FlowControl|Delay 0.2)
                  (CallFunction|PasarAOtroCamara _newpawn)))))
          (else
            (Variables|Default|SetisLooking false)
            (Variables|Default|SetTimeToteleport 0.0)))))
    (:then_2
      (if (Variables|Default|GetTimer%20activated)
        (bind _output_get_2 (Variables|Default|SetTimer (+ DeltaSeconds (Variables|Default|GetTimer))))
        (if (> _output_get_2 1.5)
          (Rendering|SetVisibility (Variables|/Game/Blueprints/Timer.Timer_C|GetTextRender _actual_timer) false false)
          (Rendering|SetVisibility (Variables|/Game/Blueprints/Timer.Timer_C|GetCube _actual_timer) false false)
          (Variables|Default|SetTimer 0.0)
          (Variables|Default|SetTimer%20activated false))))))

(event EventBeginPlay
  (Collision|SetCollisionObjectType (Variables|Default|GetStaticMesh) "ECC_GameTraceChannel1")
  (Utilities|FlowControl|Sequence
    (:then_0
      (Input|EnableInput (Game|GetPlayerController 0)))
    (:then_1
      (bind _returnvalue (UserInterface|CreateWidget "/Game/L1/Blueprints/puntoCentroPantalla.puntoCentroPantalla_C"))
      (UserInterface|Viewport|AddtoViewport _returnvalue 0))))

(event EventPossessed
  (params (NewController :type Controller%20Object%20Reference))
  ;[1 1 1] Toggle Visibility of Stiatic Mesh
  (Rendering|SetVisibility (Variables|Default|GetStaticMesh) false false)
  (Variables|Default|SetisPossessed true))

(event Input|ActionEvents|InputActionAcuse_Input
  (params (Key :type Key%20Structure :default "AnyKey"))
  (:Pressed
    (if (Variables|/Game/AI_Stuff/AI/NPCS.NPCS_C|GetisCriminal (Variables|Default|Getasd))
      (Development|PrintString "YOU WIN!")
      (Game|OpenLevel(byName) "L2map")
      (else
        (Development|PrintString "YOU LOSE")))))

(event Input|MouseEvents|MouseX
  (params (AxisValue :type Float%20%28single-precision%29))
  ;[1 1 1] Rotate Camera with Mouse
  (Class|PlayerController|AddYawInput (Game|GetPlayerController 0) AxisValue))

(event Input|MouseEvents|MouseY
  (params (AxisValue :type Float%20%28single-precision%29))
  ;[1 1 1] Rotate Camera with Mouse
  (Class|PlayerController|AddPitchInput (Game|GetPlayerController 0) (stale _result)))

(event Input|KeyboardEvents|E
  (params (Key :type Key%20Structure :default "AnyKey"))
  (bind _cube (Variables|Default|GetCube))
  (bind _actual_timer (Variables|Default|GetActual_Timer))
  (:Pressed
    (Variables|Default|SetTimer%20activated true)
    (Transformation|SetActorLocationAndRotation (Variables|Default|GetActual_Timer) (Transformation|GetWorldLocation _cube) (Transformation|GetWorldRotation _cube))
    (Rendering|SetVisibility (Variables|/Game/Blueprints/Timer.Timer_C|GetTextRender _actual_timer) true false)
    (Rendering|SetVisibility (Variables|/Game/Blueprints/Timer.Timer_C|GetCube _actual_timer) true false)))

(event Input|KeyboardEvents|SpaceBar
  (params (Key :type Key%20Structure :default "AnyKey"))
  (:Pressed
    ;[1 1 1] Aqui se activa el FadeOut
    (bind (_newpawn _canwe) (CallFunction|CanWeTransporttoCamera))
    (if _canwe
      (Variables|Default|SetTimeToteleport -0.2)
      (Utilities|FlowControl|Delay 0.2)
      (CallFunction|PasarAOtroCamara _newpawn))))

(fn ConstructionScript)

(fn PasarRotacion
  (params (posicionAnterior :type Vector))
  ;[1 1 1] La posicion de la camara vieja
  (Transformation|SetActorRotation (Math|Rotator|FindLookatRotation (Transformation|GetActorLocation) posicionAnterior)))

(fn CanWeGotoThatCamera
  (params (aLaQueVoy :type Camera%20Pawn%20Object%20Reference))
  (bind _returnvalue (Utilities|String|ToString(Object) aLaQueVoy))
  (bind _returnvalue_2 (Utilities|String|ToString(Object) aLaQueVoy))
  (bind _returnvalue_3 (Utilities|String|ToString(Object) aLaQueVoy))
  (bind _returnvalue_4 (Game|GetCurrentLevelName true))
  (switch string _returnvalue_4
    (:Default
      (return false))
    (:L1map
      (switch string (Utilities|String|ToString(Object) self)
        (:Default
          _)
        (:CameraPawn1
          ;[1 1 1] A la que voy
          (switch string _returnvalue_3
            (:Default
              _)
            (:CameraPawn2
              (return true))
            (:CameraPawn6
              (return true))
            (:CameraPawn9
              (return true))
            (:CameraPawn12
              (return true))))
        (:CameraPawn2
          (switch string _returnvalue_3
            (:Default
              _)
            (:CameraPawn1
              (return true))
            (:CameraPawn3
              (return true))
            (:CameraPawn4
              (return true))))
        (:CameraPawn3
          ;[1 1 1] L1
          (switch string _returnvalue_3
            (:Default
              _)
            (:CameraPawn2
              (return true))
            (:CameraPawn4
              (return true))))
        (:CameraPawn4
          (switch string _returnvalue_3
            (:Default
              _)
            (:CameraPawn2
              (return true))
            (:CameraPawn3
              (return true))))
        (:CameraPawn5
          (switch string _returnvalue_3
            (:Default
              _)
            (:CameraPawn8
              (return true))
            (:CameraPawn6
              (return true))
            (:CameraPawn7
              (return true))))
        (:CameraPawn6
          (switch string _returnvalue_3
            (:Default
              _)
            (:CameraPawn1
              (return true))
            (:CameraPawn5
              (return true))))
        (:CameraPawn7
          (switch string _returnvalue_3
            (:Default
              _)
            (:CameraPawn5
              (return true))))
        (:CameraPawn8
          (switch string _returnvalue_3
            (:Default
              _)
            (:CameraPawn5
              (return true))))
        (:CameraPawn9
          (switch string _returnvalue_3
            (:Default
              _)
            (:CameraPawn1
              (return true))
            (:CameraPawn10
              (return true))
            (:CameraPawn11
              (return true))))
        (:CameraPawn10
          (switch string _returnvalue_3
            (:Default
              _)
            (:CameraPawn9
              (return true))))
        (:CameraPawn11
          (switch string _returnvalue_3
            (:Default
              _)
            (:CameraPawn9
              (return true))))
        (:CameraPawn12
          (switch string _returnvalue_3
            (:Default
              _)
            (:CameraPawn1
              (return true))
            (:CameraPawn13
              (return true))
            (:CameraPawn14
              (return true))
            (:CameraPawn15
              (return true))))
        (:CameraPawn13
          (switch string _returnvalue_3
            (:Default
              _)
            (:CameraPawn12
              (return true))))
        (:CameraPawn14
          (switch string _returnvalue_3
            (:Default
              _)
            (:CameraPawn12
              (return true))))
        (:CameraPawn15
          (switch string _returnvalue_3
            (:Default
              _)
            (:CameraPawn12
              (return true)))))
      (return false))
    (:L2map
      ;[1 1 1] L2
      ;;[1 1 1] En la que estoy
      (switch string (Utilities|String|ToString(Object) self)
        (:Default
          _)
        (:CameraPawn1
          ;;[1 1 1] A la que voy
          (switch string _returnvalue_2
            (:Default
              _)
            (:CameraPawn1
              _)
            (:CameraPawn2
              ;[1 1 1] True
              (return true))
            (:CameraPawn3
              (return true))))
        (:CameraPawn2
          (switch string _returnvalue_2
            (:Default
              _)
            (:CameraPawn1
              (return true))
            (:CameraPawn2
              _)
            (:CameraPawn3
              (return true))))
        (:CameraPawn3
          (switch string _returnvalue_2
            (:Default
              _)
            (:CameraPawn1
              (return true))
            (:CameraPawn2
              (return true))
            (:CameraPawn3
              _)))))
    (:Ltutorial
      ;[1 1 1] Ltutorial
      ;;[1 1 1] En la que estoy
      (switch string (Utilities|String|ToString(Object) self)
        (:CameraPawn1
          (switch string _returnvalue
            (:Default
              _)
            (:CameraPawn3
              (return true))))
        (:CameraPawn2
          (switch string _returnvalue
            (:Default
              _)
            (:CameraPawn5
              (return true))
            (:CameraPawn3
              (return true))))
        (:CameraPawn3
          (switch string _returnvalue
            (:Default
              _)
            (:CameraPawn1
              (return true))))
        (:CameraPawn5
          (switch string _returnvalue
            (:Default
              _)
            (:CameraPawn2
              (return true)))))))
  ;[1 1 1] False
  (return false))

(fn CanWeTransporttoCamera
  (bind _returnvalue (Transformation|GetActorLocation))
  ;[1 1 1] ace bar)
  (bind _outhit (Collision|SphereTraceForObjects _returnvalue (+ _returnvalue (* (Transformation|GetActorForwardVector (Game|GetPlayerController 0)) 1e+04)) 1.5e+02 (Utilities|Array|MakeArray "ObjectTypeQuery7") false 0 "None"))
  (if (== (Utilities|GetClass (.HitActor (Collision|BreakHitResult _outhit))) "CameraPawn_C")
    (bind _ascamera_pawn (Utilities|Casting|CastToCameraPawn (.HitActor (Collision|BreakHitResult _outhit)))
      (:then
        ;[1 1 1] Miramos si podemos ir a esa camara
        (bind _canigo (CallFunction|CanWeGotoThatCamera _ascamera_pawn))
        ;[1 1 1] Le pasamos a la siguinte camara de donde venimos, para que apunte a ella
        (if _canigo
          (bind _returnvalue_2 (UserInterface|CreateWidget "/Game/UMG/fadeOut.fadeOut_C" (Game|GetPlayerController 0)))
          (UserInterface|Viewport|AddtoViewport _returnvalue_2 0)
          (bind _returnvalue_3 (AddComponent|AddAudioComponent false))
          (Audio|Components|Audio|Play _returnvalue_3 0.0)
          (return _ascamera_pawn true)
          (else
            _)))
      (:CastFailed
        _)))
  (return 0 false))

(fn PasarAOtroCamara
  (params (NewParam :type Camera%20Pawn%20Object%20Reference))
  (CallFunction|PasarRotacion NewParam (Transformation|GetActorLocation))
  (Pawn|Possess (Game|GetPlayerController 0) NewParam))